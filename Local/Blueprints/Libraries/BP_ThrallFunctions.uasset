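; Blueprint function library of helpers for thrall NPCs, each casting the thrall to BaseHumanoidNPC.
; Equipment functions strip all gear or only weapons by slot, or swap body, arm, leg and foot slots to coarse clothing item templates.
; Bearer-profession thralls get a backpack capacity scaled by tier from a base size plus a per-tier bonus.
; SetupPlacedThrall is an empty stub.
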(fn `RemoveItemsFromThrall`
  (params (Thrall :type "Actor Object Reference"))
  (locals (EquipmentInventory :type "EquipmentInventory Object Reference"))
  (bind _asbase_humanoid_npc (cast `/Game/Characters/NPCs/Humanoid/BaseHumanoidNPC` Thrall))
  (bind _output_get (set `local.EquipmentInventory` (`/Game/Characters/BaseBPChar.GetEquipmentInventory` _asbase_humanoid_npc)))
  (`|ExecutionSequence`
    (:`then_0`
      (`ItemInventory.RemoveItem` _output_get (`EquipmentInventory.GetSlotIndex` (`local.EquipmentInventory`) "MainHand")))
    (:`then_1`
      (`ItemInventory.RemoveItem` _output_get (`EquipmentInventory.GetSlotIndex` (`local.EquipmentInventory`) "OffHand")))
    (:`then_2`
      (`ItemInventory.RemoveItem` _output_get (`EquipmentInventory.GetSlotIndex` (`local.EquipmentInventory`) "DualHand")))
    (:`then_3`
      (`ItemInventory.RemoveItem` _output_get (`EquipmentInventory.GetSlotIndex` (`local.EquipmentInventory`) "Head")))
    (:`then_4`
      (`ItemInventory.RemoveItem` _output_get (`EquipmentInventory.GetSlotIndex` (`local.EquipmentInventory`) "Torso")))
    (:`then_5`
      (`ItemInventory.RemoveItem` _output_get (`EquipmentInventory.GetSlotIndex` (`local.EquipmentInventory`) "Arms")))
    (:`then_6`
      (`ItemInventory.RemoveItem` _output_get (`EquipmentInventory.GetSlotIndex` (`local.EquipmentInventory`) "Legs")))
    (:`then_7`
      (`ItemInventory.RemoveItem` _output_get (`EquipmentInventory.GetSlotIndex` (`local.EquipmentInventory`) "Feet")))))

(fn `RemoveWeaponsFromThrall`
  (params (Thrall :type "Actor Object Reference"))
  (locals (EquipmentInventory :type "EquipmentInventory Object Reference"))
  (bind _asbase_humanoid_npc (cast `/Game/Characters/NPCs/Humanoid/BaseHumanoidNPC` Thrall))
  (bind _output_get (set `local.EquipmentInventory` (`/Game/Characters/BaseBPChar.GetEquipmentInventory` _asbase_humanoid_npc)))
  (`|ExecutionSequence`
    (:`then_0`
      (`ItemInventory.RemoveItem` _output_get (`EquipmentInventory.GetSlotIndex` (`local.EquipmentInventory`) "MainHand")))
    (:`then_1`
      (`ItemInventory.RemoveItem` _output_get (`EquipmentInventory.GetSlotIndex` (`local.EquipmentInventory`) "OffHand")))
    (:`then_2`
      (`ItemInventory.RemoveItem` _output_get (`EquipmentInventory.GetSlotIndex` (`local.EquipmentInventory`) "DualHand")))))

(fn `SetBearerInventorySlots`
  (params (Thrall :type "Actor Object Reference") (Info :type "ThrallInfo Structure"))
  (locals (InventorySizeBonusPerTier :type Integer :default 5) (InventorySize :type Integer :default 10) (BearerProfession :type "EThrallProfession Enum" :default "Bearer") (InventorySizeBonus :type Integer :default 5))
  (bind (_thrallname _thrallicon _thralltier _thrallbuff _thrallprofession) (break `ThrallInfo` Info))
  (bind _asbase_humanoid_npc (cast `/Game/Characters/NPCs/Humanoid/BaseHumanoidNPC` Thrall))
  (bind _returnvalue (`ConanCharacter.GetBackpackInventory` _asbase_humanoid_npc))
  (if (== (`local.BearerProfession`) _thrallprofession)
    (`ItemInventory.SetMaxItemCount` _returnvalue (+ (* (`local.InventorySizeBonusPerTier`) (`KismetMathLibrary.Conv_ByteToInt` _thralltier)) (`local.InventorySize`)))))

(fn `SetCoarseClothingForThrall`
  (params (Thrall :type "Actor Object Reference"))
  (locals (EquipmentInventory :type "EquipmentInventory Object Reference"))
  (bind _asbase_humanoid_npc (cast `/Game/Characters/NPCs/Humanoid/BaseHumanoidNPC` Thrall))
  (bind _output_get (set `local.EquipmentInventory` (`/Game/Characters/BaseBPChar.GetEquipmentInventory` _asbase_humanoid_npc)))
  (`|ExecutionSequence`
    (:`then_0`
      (`ItemInventory.RemoveItem` _output_get (`EquipmentInventory.GetSlotIndex` (`local.EquipmentInventory`) "Torso"))
      (`EquipmentInventory.AddItemTemplateToSlot` _output_get "Torso" 52202 1 false 1.0 -1.0))
    (:`then_1`
      (`ItemInventory.RemoveItem` _output_get (`EquipmentInventory.GetSlotIndex` (`local.EquipmentInventory`) "Arms"))
      (`EquipmentInventory.AddItemTemplateToSlot` _output_get "Arms" 52203 1 false 1.0 -1.0))
    (:`then_2`
      (`ItemInventory.RemoveItem` _output_get (`EquipmentInventory.GetSlotIndex` (`local.EquipmentInventory`) "Legs"))
      (`EquipmentInventory.AddItemTemplateToSlot` _output_get "Legs" 52204 1 false 1.0 -1.0))
    (:`then_3`
      (`ItemInventory.RemoveItem` _output_get (`EquipmentInventory.GetSlotIndex` (`local.EquipmentInventory`) "Feet"))
      (`EquipmentInventory.AddItemTemplateToSlot` _output_get "Feet" 52205 1 false 1.0 -1.0))))

(fn `SetupPlacedThrall`
  (params (Thrall :type "Actor Object Reference") (Info :type "ThrallInfo Structure"))
  (return))