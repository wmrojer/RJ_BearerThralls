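; BP_BearerThrallComponent is a component that sets bearer inventory slots on its owning humanoid NPC thrall.
; While an adjustment is pending, Tick validates the owner, casts it to BaseHumanoidNPC and passes the ThrallInfo from its BP_ThrallComponent to SetBearerInventorySlots.
; It retries until that thrall component is valid or the cast fails, then deactivates itself on the following tick.
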(event `self.ReceiveTick`
  (params (DeltaSeconds :type "Float (single-precision)"))
  (if (`self.NeedsAdjustment`)
    (bind _owner (`/Game/Mods/RJ_BearerThralls/Blueprints/Libraries/BP_ComponentMacros.ValidateOwner`)
      (:`Success`
        (bind _asbase_humanoid_npc (cast `/Game/Characters/NPCs/Humanoid/BaseHumanoidNPC` _owner)
          (:`then`
            (bind _returnvalue (`Actor.GetComponentByClass` _owner "/Game/Systems/Thrall/BP_ThrallComponent.BP_ThrallComponent_C"))
            (if (`KismetSystemLibrary.IsValid` _returnvalue)
              (`/Game/Mods/RJ_BearerThralls/Blueprints/Libraries/BP_ThrallFunctions.SetBearerInventorySlots` _asbase_humanoid_npc (`ThrallComponent.ThrallInfo` _returnvalue))
              (set `self.NeedsAdjustment` false)))
          (:`CastFailed`
            (set `self.NeedsAdjustment` false)))))
    (else
      (`self.Deactivate`))))